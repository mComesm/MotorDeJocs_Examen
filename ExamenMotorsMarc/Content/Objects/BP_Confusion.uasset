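; Confusion trigger object that inverts WASD movement controls for five seconds when anything overlaps its Box.
; The overlap event removes the MoveForward and MoveRight axis mappings and re-adds them with opposite keys, then waits on a Delay before SetControlsToNormal restores them.
; The swap edits the global Input Settings at runtime with keymap rebuilds, with no check on the overlapping actor.
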(event `self.Box.OnComponentBeginOverlap`
  (params (OverlappedComponent :type "PrimitiveComponent Object Reference") (OtherActor :type "Actor Object Reference") (OtherComp :type "PrimitiveComponent Object Reference") (OtherBodyIndex :type Integer) (bFromSweep :type Boolean) (SweepResult :type "HitResult Structure (by ref)"))
  (bind _returnvalue (`InputSettings.GetInputSettings`))
  (`|ExecutionSequence`
    (:`then_0`
      (`InputSettings.RemoveAxisMapping` _returnvalue (make `InputAxisKeyMapping` "MoveForward" 1.0 "W") true)
      (`InputSettings.RemoveAxisMapping` _returnvalue (make `InputAxisKeyMapping` "MoveForward" -1.0 "S") true)
      (`InputSettings.RemoveAxisMapping` _returnvalue (make `InputAxisKeyMapping` "MoveRight" 1.0 "D") true)
      (`InputSettings.RemoveAxisMapping` _returnvalue (make `InputAxisKeyMapping` "MoveRight" -1.0 "A") true))
    (:`then_1`
      (`InputSettings.AddAxisMapping` _returnvalue (make `InputAxisKeyMapping` "MoveForward" 1.0 "S") true)
      (`InputSettings.AddAxisMapping` _returnvalue (make `InputAxisKeyMapping` "MoveForward" -1.0 "W") true)
      (`InputSettings.AddAxisMapping` _returnvalue (make `InputAxisKeyMapping` "MoveRight" 1.0 "A") true)
      (`InputSettings.AddAxisMapping` _returnvalue (make `InputAxisKeyMapping` "MoveRight" -1.0 "D") true)
      (`KismetSystemLibrary.Delay` 5.0)
      (`self.SetControlsToNormal`))))

(fn `SetControlsToNormal`
  (bind _returnvalue (`InputSettings.GetInputSettings`))
  (`|ExecutionSequence`
    (:`then_0`
      (`InputSettings.RemoveAxisMapping` _returnvalue (make `InputAxisKeyMapping` "MoveForward" -1.0 "W") true)
      (`InputSettings.RemoveAxisMapping` _returnvalue (make `InputAxisKeyMapping` "MoveForward" 1.0 "S") true)
      (`InputSettings.RemoveAxisMapping` _returnvalue (make `InputAxisKeyMapping` "MoveRight" -1.0 "D") true)
      (`InputSettings.RemoveAxisMapping` _returnvalue (make `InputAxisKeyMapping` "MoveRight" 1.0 "A") true))
    (:`then_1`
      (`InputSettings.AddAxisMapping` _returnvalue (make `InputAxisKeyMapping` "MoveForward" -1.0 "S") true)
      (`InputSettings.AddAxisMapping` _returnvalue (make `InputAxisKeyMapping` "MoveForward" 1.0 "W") true)
      (`InputSettings.AddAxisMapping` _returnvalue (make `InputAxisKeyMapping` "MoveRight" -1.0 "A") true)
      (`InputSettings.AddAxisMapping` _returnvalue (make `InputAxisKeyMapping` "MoveRight" 1.0 "D") true))))

(fn `UserConstructionScript`)